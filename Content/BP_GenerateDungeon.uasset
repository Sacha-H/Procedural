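; Procedural dungeon generator actor that assembles random room meshes in its construction script, up to MaxRoomNumber.
; A queue seeded with the actor transform holds open exits, expanded breadth-first through CreateRoom.
; Each room mesh comes from a random DT_RoomsPreset row and attaches to its parent room at that exit.
; Rooms overlapping WorldStatic components other than their parent are destroyed, while accepted rooms queue their endpoints and mark them with arrows.
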(event EventBeginPlay)

(event Collision|EventActorBeginOverlap
  (params (OtherActor :type Actor%20Object%20Reference)))

(event EventTick
  (params (DeltaSeconds :type Float%20%28single-precision%29)))

(fn ConstructionScript
  (bind _returnvalue (Transformation|GetActorTransform))
  (bind _queue (Variables|Default|GetQueue))
  (Utilities|Array|Clear _queue)
  (Utilities|Array|Add _queue (Utilities|Struct|MakeSEndPointInfo (.location _returnvalue) (.rotation _returnvalue) 0))
  (CallFunction|CreateRoom true)
  (while (and (Utilities|Array|IsNotEmpty (Variables|Default|GetQueue)) (< (Variables|Default|GetCurrentNbRoomSpawn) (Variables|Default|GetMaxRoomNumber)))
    (CallFunction|CreateRoom false)))

(fn CreateRoom
  (params (FirstRoom :type Boolean))
  (bind _queue (Variables|Default|GetQueue))
  (bind _output (Utilities|Array|Get(acopy) _queue))
  (bind _outrownames (DataTable|GetDataTableRowNames "/Game/DT_RoomsPreset.DT_RoomsPreset"))
  (bind _returnvalue (Utilities|GetDataTableRow "/Game/DT_RoomsPreset.DT_RoomsPreset" (.OutItem (Utilities|Array|Random _outrownames)))
    (:then
      (bind _returnvalue_2 (AddComponent|AddStaticMeshComponent true (Math|Transform|MakeTransform (.location _output) (.rotation _output) "1.000000,1.000000,1.000000")))
      (if FirstRoom
        _
        (else
          (Transformation|AttachComponentToComponent _returnvalue_2 (.parentmeshcomponent _output) "None" "KeepRelative" "KeepRelative" "KeepRelative" true)))
      (Components|StaticMesh|SetStaticMesh _returnvalue_2 (.roommesh _returnvalue))
      (bind _outcomponents (Class|KismetSystemLibrary|ComponentOverlapComponents _returnvalue_2 (Transformation|GetWorldTransform _returnvalue_2) (Utilities|Array|MakeArray "ObjectTypeQuery1")))
      (for _array_element _outcomponents
        (if (!= _array_element (.parentmeshcomponent _output))
          (Development|PrintString (Utilities|String|Append (Utilities|GetDisplayName _returnvalue_2) " overlap " (Utilities|GetDisplayName _array_element)))
          (LocalVariables|SetFoundOne true)))
      (Utilities|Array|RemoveIndex (Variables|Default|GetQueue))
      (if (LocalVariables|GetFoundOne)
        (Components|DestroyComponent _returnvalue_2)
        (else
          (Math|Integer|IncrementInt (Variables|Default|GetCurrentNbRoomSpawn)
            (:%20%20
              (for _array_element_2 (.endpoint _returnvalue)
                (Utilities|Array|Add (Variables|Default|GetQueue) (Utilities|Struct|MakeSEndPointInfo (.Location (Utilities|Struct|BreakSEndPointInfo _array_element_2)) (.Rotation (Utilities|Struct|BreakSEndPointInfo _array_element_2)) _returnvalue_2))
                (bind _returnvalue_3 (AddComponent|AddArrowComponent true (Math|Transform|MakeTransform (.Location (Utilities|Struct|BreakSEndPointInfo _array_element_2)) (.Rotation (Utilities|Struct|BreakSEndPointInfo _array_element_2)) "1.000000,1.000000,1.000000")))
                (Transformation|AttachComponentToComponent _returnvalue_3 _returnvalue_2 "None" "KeepRelative" "KeepRelative" "KeepRelative" true)))))))))